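; Tower defense projectile that homes in on its EnemyTarget, drawn as a billboard sprite set from ProjectileTexture at construction.
; Each Tick it sweeps from its current location toward the target by a growing LerpAlpha, so the homing tightens over time and depends on frame rate.
; It destroys itself on reaching the target's location, when Hitsphere overlaps that target, or after a short lifetime, and applies no damage here.
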(event OnComponentBeginOverlap(Hitsphere)
  (params (OverlappedComponent :type Primitive%20Component%20Object%20Reference) (OtherActor :type Actor%20Object%20Reference) (OtherComp :type Primitive%20Component%20Object%20Reference) (OtherBodyIndex :type Integer) (bFromSweep :type Boolean) (SweepResult :type Hit%20Result%20Structure%20%28by%20ref%29))
  (bind _asenemy_character (Utilities|Casting|CastToEnemyCharacter OtherActor))
  (if (== _asenemy_character (Variables|Default|GetEnemyTarget))
    (Actor|DestroyActor)))

(event EventBeginPlay
  (Utilities|FlowControl|Delay 2.0)
  (if (Utilities|IsValid self)
    (Actor|DestroyActor)))

(event Collision|EventActorBeginOverlap
  (params (OtherActor :type Actor%20Object%20Reference)))

(event EventTick
  (params (DeltaSeconds :type Float%20%28single-precision%29))
  (bind _self self)
  (bind _self_2 self)
  (bind _enemytarget (Variables|Default|GetEnemyTarget))
  ;[1 1 1] Lerp towards enemy
  (if (Utilities|IsValid _enemytarget)
    (Transformation|SetActorLocation _self_2 (Math|Vector|Lerp(Vector) (Transformation|GetActorLocation _self_2) (Transformation|GetActorLocation _enemytarget) (Variables|Default|GetLerpAlpha)) true false)
    (Variables|Default|SetLerpAlpha (+ (Variables|Default|GetLerpAlpha) 0.005))
    ;[1 1 1] Destroy self if location is close to destination
    (if (Utilities|IsValid _self)
      (if (Math|Vector|Equal(Vector) (Transformation|GetActorLocation _self) (Transformation|GetActorLocation (Variables|Default|GetEnemyTarget)) 0.001)
        (Actor|DestroyActor)))))

(fn ConstructionScript
  (Rendering|Components|Sprite|SetSprite (Variables|Default|GetBillboard) (Variables|Default|GetProjectileTexture)))