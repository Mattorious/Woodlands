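; Roguelike item spawner actor that has a one-in-four chance to place a random weapon when play begins.
; On BeginPlay it rolls a random integer modulo four, then spawns a uniformly chosen class from its Weapons array at its own transform.
; The construction script, overlap and tick events are empty.
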(event EventBeginPlay
  (bind _weapons (Variables|Default|GetWeapons))
  ;[1 1 1] 25% Chance to spawn an item
  (if (== (Math|Integer|%(Integer) (Math|Random|RandomInteger 1000) 4) 0)
    (Game|SpawnActorfromClass (Utilities|Array|Get(acopy) _weapons (Math|Random|RandomIntegerinRange 0 (- (Utilities|Array|Length _weapons) 1))) (Transformation|GetActorTransform self) "Undefined" 0 0)))

(event Collision|EventActorBeginOverlap
  (params (OtherActor :type Actor%20Object%20Reference)))

(event EventTick
  (params (DeltaSeconds :type Float%20%28single-precision%29)))

(fn ConstructionScript)