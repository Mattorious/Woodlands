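; Tile manager that builds a randomized level layout at BeginPlay by rearranging the actors in its Tiles array.
; GenerateLevelLayout shuffles the tiles, then teleports each to a computed position with a random rotation from PossibleRotations.
; CalculateNextPosition runs a random walk from the origin, adding random PossibleTransformations offsets and rerolling against PreviousPositions to avoid overlaps.
; The reroll has no retry limit, and debug prints log positions and separately rolled rotations.
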(event EventBeginPlay
  (CallFunction|GenerateLevelLayout))

(event Collision|EventActorBeginOverlap
  (params (OtherActor :type Actor%20Object%20Reference)))

(event EventTick
  (params (DeltaSeconds :type Float%20%28single-precision%29)))

(fn ConstructionScript)

(fn CalculateNextPosition
  (params (CurrentPosition :type Vector) (ForIndex :type Integer))
  (if (== ForIndex 0)
    (Variables|Default|SetDesiredPosition "0, 0, 0")
    (else
      (while (Utilities|Array|ContainsItem (Variables|Default|GetPreviousPositions) (stale _generatedpos)) :!label _label
        (bind _generatedpos (CallFunction|GenerateNewValue (Variables|Default|GetDesiredPosition)))
        (goto _label))
      (bind _output_get (Variables|Default|SetDesiredPosition _generatedpos))))
  (Development|PrintString (Utilities|String|ToString(Vector) _output_get))
  (Utilities|Array|Add (Variables|Default|GetPreviousPositions) _output_get)
  (return _output_get))

(fn GenerateNewValue
  (params (LastPos :type Vector))
  (return (+ LastPos (Utilities|Array|Get(acopy) (Variables|Default|GetPossibleTransformations) (Math|Random|RandomIntegerinRange 0 3)))))

(fn GenerateLevelLayout
  (bind _returnvalue (Math|Random|RandomIntegerinRange 0 3))
  (bind _tiles (Variables|Default|GetTiles))
  (bind _possiblerotations (Variables|Default|GetPossibleRotations))
  (bind _output (Utilities|Array|Get(acopy) _possiblerotations _returnvalue))
  (Variables|Default|SetPreviousPositions (Utilities|Array|MakeArray))
  (Utilities|Array|Shuffle _tiles)
  (for (_array_element _array_index) _tiles
    (bind _nextpos (CallFunction|CalculateNextPosition (Variables|Default|GetDesiredPosition) _array_index))
    (bind _output_get (Variables|Default|SetDesiredPosition _nextpos))
    (Transformation|Teleport _array_element _output_get _output)
    (Development|PrintString (Utilities|String|ToString(Rotator) _output))))