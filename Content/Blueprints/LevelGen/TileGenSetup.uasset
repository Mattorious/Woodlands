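; TileGenSetup is an unfinished level generation Blueprint that passes each tile's location to CalculateNextPosition on BeginPlay.
; The function is built as a random walk, adding one of four offsets and retrying against PreviousPositions, though its final pick is re-rolled unchecked.
; BeginPlay always passes index 0, so every result is the origin.
; Results are printed and recorded, but no tile is moved.
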(event EventBeginPlay
  (for _array_element (Variables|Default|GetTiles)
    (CallFunction|CalculateNextPosition (Transformation|GetActorLocation _array_element))))

(event Collision|EventActorBeginOverlap
  (params (OtherActor :type Actor%20Object%20Reference)))

(event EventTick
  (params (DeltaSeconds :type Float%20%28single-precision%29)))

(fn ConstructionScript)

(fn CalculateNextPosition
  (params (CurrentPos :type Vector) (CurrentForLoopIndex :type Integer))
  (bind _returnvalue (Math|Random|RandomIntegerinRange 0 3))
  (bind _possibletransformations (Variables|Default|GetPossibleTransformations))
  (bind _output (Utilities|Array|Get(acopy) _possibletransformations _returnvalue))
  (bind _returnvalue_2 (+ CurrentPos _output))
  (if (== CurrentForLoopIndex 0)
    (Variables|Default|SetDesiredPosition "0, 0, 0")
    (else
      (while (Utilities|Set|Contains (Variables|Default|GetPreviousPositions) _returnvalue_2)
        _)
      (bind _output_get (Variables|Default|SetDesiredPosition _returnvalue_2))))
  (Development|PrintString (Utilities|String|ToString(Vector) _output_get))
  (Utilities|Set|Add (Variables|Default|GetPreviousPositions) _output_get)
  (return _output_get))