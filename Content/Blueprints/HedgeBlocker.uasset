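; HedgeBlocker is an actor that forms a hedge of shrubs with a box collision volume, sized by a Length value.
; The construction script sizes and offsets the box from BlockerVolume bounds, using Length as its Y extent.
; It then adds shrub mesh components at fixed steps along Y, their count derived from Length, with random X jitter, scale and yaw.
; The event graph holds no active logic.
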(event EventBeginPlay)

(event Collision|EventActorBeginOverlap
  (params (OtherActor :type Actor%20Object%20Reference)))

(event EventTick
  (params (DeltaSeconds :type Float%20%28single-precision%29)))

(fn ConstructionScript
  (bind _blockervolume (Variables|Default|GetBlockerVolume))
  (bind _length (Variables|Default|GetLength))
  (bind _box (Variables|Default|GetBox))
  (bind (_origin _boxextent) (Math|BoxSphereBounds|BreakBoxSphereBounds _blockervolume))
  (bind (_x _y _z) (Math|Vector|BreakVector _boxextent))
  (bind (_x_2 _y_2) (Math|Vector|BreakVector _origin))
  ;[1 1 1] Constructing collision box
  (Components|Box|SetBoxExtent _box (Math|Vector|MakeVector _x _length _z) true)
  (Transformation|AddLocalOffset _box (Math|Vector|MakeVector _x_2 _y_2 _z) false false)
  ;[1 1 1] Adding shrubs
  (for _index (range 0 (- (Math|Float|Truncate (/ _length 42.0)) 1))
    (bind _returnvalue (AddComponent|AddStaticMeshComponent false))
    (Components|StaticMesh|SetStaticMesh _returnvalue (Variables|Default|GetShrubMesh))
    (Transformation|AddWorldOffset _returnvalue (Math|Vector|MakeVector (Math|Random|RandomFloatinRange -5e+01 5e+01) (- _length (LocalVariables|GetShrubOffset)) 0.0) false false)
    (LocalVariables|SetShrubOffset (+ (LocalVariables|GetShrubOffset) 1e+02))
    (Transformation|SetRelativeScale3D _returnvalue (* (Variables|/Script/Engine.SceneComponent|GetRelativeScale3D _returnvalue) (Math|Random|RandomFloatinRange 0.9 1.2)))
    (Transformation|SetRelativeRotation _returnvalue (Math|Rotator|MakeRotator 0.0 0.0 (Math|Random|RandomFloatinRange 0.0 359.0)) false false)))