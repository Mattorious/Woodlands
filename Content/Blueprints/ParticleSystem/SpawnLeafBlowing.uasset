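; Trigger-box actor that spawns Niagara leaf effects once the TopDownCharacter enters its box.
; Begin overlap starts a loop that waits a random few seconds, then spawns an enlarged leaf system at a random point within the box's extent, centered on world origin rather than the actor.
; End overlap also sets CharacterIsInBounds to true, so the loop keeps running after the character leaves.
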(event OnComponentBeginOverlap(Box)
  (params (OverlappedComponent :type Primitive%20Component%20Object%20Reference) (OtherActor :type Actor%20Object%20Reference) (OtherComp :type Primitive%20Component%20Object%20Reference) (OtherBodyIndex :type Integer) (bFromSweep :type Boolean) (SweepResult :type Hit%20Result%20Structure%20%28by%20ref%29))
  (if (== (Utilities|GetClass (stale OnComponentEndOverlap(Box) OtherActor)) "/Game/Blueprints/Roguelike/Character/Player/TopDownCharacter.TopDownCharacter_C")
    (bind _output_get (Variables|Default|SetCharacterIsInBounds true))
    (if _output_get :!label _label
      (Utilities|FlowControl|Delay (Math|Random|RandomFloatinRange 1.0 4.0))
      (Niagara|SpawnSystematLocation (Variables|Default|GetNiagaraLeaves) (Math|Random|RandomPointinBoundingBox "0, 0, 0" (Variables|/Script/Engine.BoxComponent|GetBoxExtent (Variables|Default|GetBox))) "0, 0,0.000000" (* (Math|Vector|MakeVector 1.0 1.0 1.0) 5.0))
      (goto _label))))

(event OnComponentEndOverlap(Box)
  (params (OverlappedComponent :type Primitive%20Component%20Object%20Reference) (OtherActor :type Actor%20Object%20Reference) (OtherComp :type Primitive%20Component%20Object%20Reference) (OtherBodyIndex :type Integer))
  (if (== (Utilities|GetClass OtherActor) "/Game/Blueprints/Roguelike/Character/Player/TopDownCharacter.TopDownCharacter_C")
    (Variables|Default|SetCharacterIsInBounds true)))

(event EventBeginPlay)

(event Collision|EventActorBeginOverlap
  (params (OtherActor :type Actor%20Object%20Reference)))

(event EventTick
  (params (DeltaSeconds :type Float%20%28single-precision%29)))

(fn ConstructionScript)