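; Campfire audio Blueprint that plays a campfire sound while the player is inside its collision box.
; When the player character begins overlapping the box, it spawns the sound at the stored campfire location.
; When the player leaves, it stops that spawned audio component after a configurable delay.
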(event OnComponentBeginOverlap(CollisionBox)
  (params (OverlappedComponent :type Primitive%20Component%20Object%20Reference) (OtherActor :type Actor%20Object%20Reference) (OtherComp :type Primitive%20Component%20Object%20Reference) (OtherBodyIndex :type Integer) (bFromSweep :type Boolean) (SweepResult :type Hit%20Result%20Structure%20%28by%20ref%29))
  ;[1 1 1] Plays the campfire sound cue when the player overlaps the collison box.
  (if (== (Game|GetPlayerCharacter 0) OtherActor)
    (bind _returnvalue (Audio|SpawnSoundatLocation (Variables|Default|GetSound) (Variables|Default|GetCampfireLocation) "0, 0, 0" 1.0 1.0 0.0 0 0))))

(event OnComponentEndOverlap(CollisionBox)
  (params (OverlappedComponent :type Primitive%20Component%20Object%20Reference) (OtherActor :type Actor%20Object%20Reference) (OtherComp :type Primitive%20Component%20Object%20Reference) (OtherBodyIndex :type Integer))
  ;[1 1 1] Plays the campfire sound cue when the player overlaps the collison box.
  (if (== OtherActor (Game|GetPlayerCharacter 0))
    (Audio|Components|Audio|StopDelayed (stale OnComponentBeginOverlap(CollisionBox) _returnvalue) (Variables|Default|GetSoundStopDelay))))

(fn ConstructionScript)