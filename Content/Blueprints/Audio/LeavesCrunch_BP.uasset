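; An audio trigger Blueprint that plays a leaves crunch sound when the player overlaps its collision box.
; Begin overlap passes through a DoOnce before checking for the player character, so any overlapping actor consumes it, then plays the sound in 2D only for the player.
; The player leaving the box resets the DoOnce after a fixed delay, acting as a cooldown.
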(event OnComponentBeginOverlap(CollisionBox)
  (params (OverlappedComponent :type Primitive%20Component%20Object%20Reference) (OtherActor :type Actor%20Object%20Reference) (OtherComp :type Primitive%20Component%20Object%20Reference) (OtherBodyIndex :type Integer) (bFromSweep :type Boolean) (SweepResult :type Hit%20Result%20Structure%20%28by%20ref%29))
  ;[1 1 1] Plays the leaves crunch sound cue when the player overlaps the collison box.
  (Utilities|FlowControl|DoOnce false
    (:Completed
      (if (== (Game|GetPlayerCharacter 0) OtherActor)
        (Audio|PlaySound2D (Variables|Default|GetSound) 1.0 1.0 0.0 0 0)))))

(event OnComponentEndOverlap(CollisionBox)
  (params (OverlappedComponent :type Primitive%20Component%20Object%20Reference) (OtherActor :type Actor%20Object%20Reference) (OtherComp :type Primitive%20Component%20Object%20Reference) (OtherBodyIndex :type Integer))
  ;[1 1 1] Plays the leaves crunch sound cue when the player overlaps the collison box.
  (if (== (Game|GetPlayerCharacter 0) OtherActor)
    (Utilities|FlowControl|Delay 1e+01)
    (Utilities|FlowControl|DoOnce false) ; enters at Reset
  ))

(fn ConstructionScript)