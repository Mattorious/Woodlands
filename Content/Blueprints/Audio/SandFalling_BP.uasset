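; Audio trigger Blueprint that plays a sand-falling sound when the player character steps into its collision box.
; Begin overlap spawns the sound at SandLocation and immediately schedules it to stop after one second with StopDelayed.
; End overlap calls the same delayed stop on the most recently spawned audio component.
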(event OnComponentBeginOverlap(Box)
  (params (OverlappedComponent :type Primitive%20Component%20Object%20Reference) (OtherActor :type Actor%20Object%20Reference) (OtherComp :type Primitive%20Component%20Object%20Reference) (OtherBodyIndex :type Integer) (bFromSweep :type Boolean) (SweepResult :type Hit%20Result%20Structure%20%28by%20ref%29))
  ;[1 1 1] Plays the Sand Falling audio file when the player steps on the collision box.
  (if (== OtherActor (Game|GetPlayerCharacter 0))
    (bind _returnvalue (Audio|SpawnSoundatLocation (Variables|Default|GetSound) (Variables|Default|GetSandLocation) "0, 0, 0" 1.0 1.0 0.0 0 0))
    (Audio|Components|Audio|StopDelayed _returnvalue 1.0)))

(event OnComponentEndOverlap(Box)
  (params (OverlappedComponent :type Primitive%20Component%20Object%20Reference) (OtherActor :type Actor%20Object%20Reference) (OtherComp :type Primitive%20Component%20Object%20Reference) (OtherBodyIndex :type Integer))
  ;[1 1 1] Plays the Sand Falling audio file when the player steps on the collision box.
  (if (== OtherActor (Game|GetPlayerCharacter 0))
    (Audio|Components|Audio|StopDelayed (stale OnComponentBeginOverlap(Box) _returnvalue) 1.0)))

(fn ConstructionScript)