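; Day-cycle Blueprint that animates the sun and skydome over a configurable day length in minutes.
; BeginPlay converts that length into seconds per game hour, which Tick uses to advance Hour and derive the sun's pitch.
; Each tick rotates the Sun actor and refreshes the Skydome's sun direction.
; From hour 20 onward a fixed rotation overrides the sun, as Hour keeps increasing without wrapping.
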(event EventBeginPlay
  (bind _output_get (Variables|Default|Set1Day (* (Variables|Default|GetDayLengthinMinutes) 6e+01)))
  (Variables|Default|Set1Hour (/ _output_get 24.0)))

(event Collision|EventActorBeginOverlap
  (params (OtherActor :type Actor%20Object%20Reference)))

(event EventTick
  (params (DeltaSeconds :type Float%20%28single-precision%29))
  ;[1 1 1] Increasing Hour and Sun Angle
  (bind _output_get (Variables|Default|SetHour (+ (Variables|Default|GetHour) (/ DeltaSeconds (Variables|Default|Get1Hour)))))
  (bind _output_get_2 (Variables|Default|SetSunAngle (+ (* (/ _output_get 6.0) 9e+01) 9e+01)))
  (Transformation|SetActorRotation (Variables|Default|GetSun) (Math|Rotator|MakeRotator 0.0 _output_get_2 3e+01))
  (Default|UpdateSunDirection (Variables|Default|GetSkydome))
  (if (>= (Variables|Default|GetHour) 2e+01)
    (Transformation|SetActorRotation (Variables|Default|GetSun) "25.000000, 0,0.000000")
    (Default|UpdateSunDirection (Variables|Default|GetSkydome))))

(fn ConstructionScript)