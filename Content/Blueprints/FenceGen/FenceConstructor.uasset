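; FenceConstructor is an actor that spawns one instance of its Model class at its Box component's transform.
; The construction script sizes the Box from BoxBounds.
; One second after BeginPlay it spawns the model, then traces WorldDynamic objects toward a fixed point on negative Y, with no start point set.
; A hit moves the spawned actor to the impact point, while a miss prints "No hit!".
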(event EventBeginPlay
  (Utilities|FlowControl|Delay 1.0)
  (bind _returnvalue (Game|SpawnActorfromClass (Variables|Default|GetModel) (Transformation|GetWorldTransform (Variables|Default|GetBox)) "Undefined" 0 0))
  (bind (_outhit _returnvalue_2) (Collision|LineTraceForObjects "0, 0, 0" "0,-500.000000, 0" (Utilities|Array|MakeArray "ObjectTypeQuery2") false 0 "None"))
  (if _returnvalue_2
    (Transformation|SetActorLocation _returnvalue (.ImpactPoint (Collision|BreakHitResult _outhit)) false false)
    (else
      (Development|PrintString "No hit!"))))

(fn ConstructionScript
  (Components|Box|SetBoxExtent (Variables|Default|GetBox) (Variables|Default|GetBoxBounds) true))