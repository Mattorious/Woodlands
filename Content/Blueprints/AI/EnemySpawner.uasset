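; Portal spawner that releases random enemies once the player comes near, then shrinks away and destroys itself.
; Its point budget is the game instance's current difficulty plus a small random bonus, recalculated when difficulty changes.
; A delayed loop spawns from AvailableEnemies until SpawnPoints reaches that budget, charging a separately randomized class's cost per spawn.
; Tick handles proximity and portal shrinking, then forces garbage collection after destruction.
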(event EventBeginPlay
  (bind _asinstance_persist (Utilities|Casting|CastToInstancePersist (Game|GetGameInstance)))
  (Variables|Default|SetMaxSpawnAvailable (+ (Variables|/Game/PersistentAssets/InstancePersist.InstancePersist_C|GetCurrentDifficulty _asinstance_persist) (Math|Random|RandomIntegerinRange 0 2)))
  (Variables|Default|SetKnownDifficulty (Variables|/Game/PersistentAssets/InstancePersist.InstancePersist_C|GetCurrentDifficulty _asinstance_persist)))

(event EventTick
  (params (DeltaSeconds :type Float%20%28single-precision%29))
  (bind _returnvalue (Game|GetPlayerCharacter 0))
  (bind _self self)
  (bind _portal (Variables|Default|GetPortal))
  (bind _availableenemies (Variables|Default|GetAvailableEnemies))
  (bind _returnvalue_2 (Utilities|Array|Length _availableenemies))
  (bind _returnvalue_3 (Transformation|GetWorldScale _portal))
  (bind _returnvalue_4 (Transformation|GetActorLocation _self))
  (bind _returnvalue_5 (- _returnvalue_2 1))
  (bind (_x _y _z) (Math|Vector|BreakVector _returnvalue_4))
  (bind _returnvalue_6 (Math|Random|RandomIntegerinRange 0 _returnvalue_5))
  (bind _output (Utilities|Array|Get(acopy) _availableenemies _returnvalue_6))
  (bind _asinstance_persist (Utilities|Casting|CastToInstancePersist (Game|GetGameInstance)))
  (if (!= (Variables|Default|GetKnownDifficulty) (Variables|/Game/PersistentAssets/InstancePersist.InstancePersist_C|GetCurrentDifficulty _asinstance_persist))
    (bind _asinstance_persist_2 (Utilities|Casting|CastToInstancePersist (Game|GetGameInstance)))
    (Variables|Default|SetMaxSpawnAvailable (+ (Variables|/Game/PersistentAssets/InstancePersist.InstancePersist_C|GetCurrentDifficulty _asinstance_persist_2) (Math|Random|RandomIntegerinRange 0 2)))
    (Variables|Default|SetKnownDifficulty (Variables|/Game/PersistentAssets/InstancePersist.InstancePersist_C|GetCurrentDifficulty _asinstance_persist_2))
    (elif (Variables|Default|GetDoneSpawning)
      (Transformation|SetWorldScale3D _portal (* _returnvalue_3 0.95))
      (if (< (.X (Math|Vector|BreakVector _returnvalue_3)) 0.05)
        (Actor|DestroyActor)
        (Utilities|Platform|CollectGarbage))
      (elif (Utilities|IsValid _returnvalue)
        (if (< (Math|Vector|Distance(Vector) _returnvalue_4 (Transformation|GetActorLocation _returnvalue)) 2.5e+03)
          (Utilities|FlowControl|DoOnce false
            (:Completed
              (if (< (Variables|Default|GetSpawnPoints) (Variables|Default|GetMaxSpawnAvailable)) :!label _label
                (Game|SpawnActorfromClass _output (Math|Transform|MakeTransform (Math|Vector|MakeVector _x _y (+ _z 1e+02))) "Undefined" 0 0)
                (Variables|Default|SetSpawnPoints (+ (Variables|Default|GetSpawnPoints) (.SpawnPoints (Utilities|GetClassDefaults _output))))
                (Utilities|FlowControl|Delay (Math|Random|RandomFloatinRange 0.5 1.5))
                (goto _label)
                (else
                  (Utilities|FlowControl|DoOnce false
                    (:Completed
                      (Variables|Default|SetDoneSpawning true))))))))))))

(fn ConstructionScript)