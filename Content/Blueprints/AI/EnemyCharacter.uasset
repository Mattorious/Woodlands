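; Enemy character Blueprint that flashes a damage material when its Health changes and destroys itself once Health reaches zero or below.
; BeginPlay caches Health and the Sphere's default material.
; Tick polls Health against LastHealth, swaps in the damage material, then after a short Delay restores the default and updates LastHealth.
; The death check runs only when both values match, so destruction follows the flash.
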(event EventBeginPlay
  (Variables|Default|SetLastHealth (Variables|Default|GetHealth))
  (Variables|Default|SetDefaultMaterial (Utilities|Array|Get(acopy) (Rendering|Material|GetMaterials (Variables|Default|GetSphere)))))

(event Collision|EventActorBeginOverlap
  (params (OtherActor :type Actor%20Object%20Reference)))

(event EventTick
  (params (DeltaSeconds :type Float%20%28single-precision%29))
  (if (!= (Variables|Default|GetHealth) (Variables|Default|GetLastHealth))
    (Rendering|Material|SetMaterial (Variables|Default|GetSphere) 0 (Variables|Default|GetDamageMaterial))
    (Utilities|FlowControl|Delay 0.5)
    (Rendering|Material|SetMaterial (Variables|Default|GetSphere) 0 (Variables|Default|GetDefaultMaterial))
    (Variables|Default|SetLastHealth (Variables|Default|GetHealth) :!label _label)
    (elif (<= (Variables|Default|GetHealth) 0)
      (Actor|DestroyActor)
      (else
        (goto _label)))))

(fn ConstructionScript)