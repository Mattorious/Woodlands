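; FindPlayer is a behavior tree task that sets or clears the player as the AI's blackboard target based on distance.
; On execute, it prints the controlled pawn's distance to player pawn 0 and compares it with SearchRadius.
; When the distance is at or beyond the radius, it stores the player and sets the in-range flag true; closer distances clear both.
; Both branches finish successfully.
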(event EventReceiveExecuteAI
  (params (OwnerController :type AI%20Controller%20Object%20Reference) (ControlledPawn :type Pawn%20Object%20Reference))
  (bind _returnvalue (Game|Player|GetPlayerPawn 0))
  (bind _inrangeboolkey (Variables|Default|GetInRangeBoolKey))
  (bind _returnvalue_2 (Transformation|GetDistanceTo ControlledPawn _returnvalue))
  (Development|PrintString (Utilities|String|ToString(Float) _returnvalue_2))
  (if (<= (Variables|Default|GetSearchRadius) _returnvalue_2)
    (Class|BTFunctionLibrary|SetBlackboardValueasObject (Variables|Default|GetTargetKey) (Game|Player|GetPlayerPawn 0))
    (Class|BTFunctionLibrary|SetBlackboardValueasBool _inrangeboolkey true)
    (AI|BehaviorTree|FinishExecute true)
    (else
      (Class|BTFunctionLibrary|ClearBlackboardValue (Variables|Default|GetTargetKey))
      (Class|BTFunctionLibrary|SetBlackboardValueasBool _inrangeboolkey false)
      (AI|BehaviorTree|FinishExecute true))))